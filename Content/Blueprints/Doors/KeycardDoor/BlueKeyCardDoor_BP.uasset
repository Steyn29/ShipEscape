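; Sliding door that opens for a third-person character holding the blue key.
; The Trigger overlap plays sounds, fires two steam effects and runs a Timeline that lerps the door between closed and open, reversing on exit.
; Without the key it plays an invalid-action sound.
; A separate Texttrigger turns the light green for key holders or shows a KeycardDoor widget otherwise, removing that widget on exit.
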(event OnComponentBeginOverlap(Trigger)
  (params (OverlappedComponent :type Primitive%20Component%20Object%20Reference) (OtherActor :type Actor%20Object%20Reference) (OtherComp :type Primitive%20Component%20Object%20Reference) (OtherBodyIndex :type Integer) (bFromSweep :type Boolean) (SweepResult :type Hit%20Result%20Structure%20%28by%20ref%29))
  (bind _asbp_third_person_character (Utilities|Casting|CastToBP_ThirdPersonCharacter OtherActor))
  (if (Variables|/Game/ThirdPerson/Blueprints/BP_ThirdPersonCharacter.BP_ThirdPersonCharacter_C|GetHasBlueKey? _asbp_third_person_character)
    (Audio|PlaySound2D "/Engine/VREditor/Sounds/UI/Selection_Changes.Selection_Changes" 1.0 1.0 0.0 0 0)
    (Components|Activation|Activate (Variables|Default|GetSteamDoor) false)
    (Audio|PlaySound2D "/Engine/VREditor/Sounds/UI/Dockable_Window_Open.Dockable_Window_Open" 1.0 1.0 0.0 0 0)
    (bind _doorposition (Timeline|Timeline Play)
      (:Update
        (Transformation|SetRelativeLocation (Variables|Default|GetDoor_Small_A) (Math|Vector|Lerp(Vector) (Variables|Door|GetDoorClosed) (Variables|Door|GetDoorOpen) _doorposition) false false)))
    (else
      (Audio|PlaySound2D "/Engine/VREditor/Sounds/UI/Invalid_Action.Invalid_Action" 1.0 1.0 0.0 0 0))))

(event OnComponentEndOverlap(Trigger)
  (params (OverlappedComponent :type Primitive%20Component%20Object%20Reference) (OtherActor :type Actor%20Object%20Reference) (OtherComp :type Primitive%20Component%20Object%20Reference) (OtherBodyIndex :type Integer))
  (bind _asbp_third_person_character (Utilities|Casting|CastToBP_ThirdPersonCharacter OtherActor))
  (if (Variables|/Game/ThirdPerson/Blueprints/BP_ThirdPersonCharacter.BP_ThirdPersonCharacter_C|GetHasBlueKey? _asbp_third_person_character)
    (Audio|PlaySound2D "/Engine/VREditor/Sounds/UI/Dockable_Window_Close.Dockable_Window_Close" 1.0 1.0 0.0 0 0)
    (bind _doorposition (Timeline|Timeline Reverse)
      (:Update
        (Transformation|SetRelativeLocation (Variables|Default|GetDoor_Small_A) (Math|Vector|Lerp(Vector) (Variables|Door|GetDoorClosed) (Variables|Door|GetDoorOpen) _doorposition) false false)))))

(event OnComponentBeginOverlap(texttrigger)
  (params (OverlappedComponent :type Primitive%20Component%20Object%20Reference) (OtherActor :type Actor%20Object%20Reference) (OtherComp :type Primitive%20Component%20Object%20Reference) (OtherBodyIndex :type Integer) (bFromSweep :type Boolean) (SweepResult :type Hit%20Result%20Structure%20%28by%20ref%29))
  (bind _asbp_third_person_character (Utilities|Casting|CastToBP_ThirdPersonCharacter OtherActor))
  (if (Variables|/Game/ThirdPerson/Blueprints/BP_ThirdPersonCharacter.BP_ThirdPersonCharacter_C|GetHasBlueKey? _asbp_third_person_character)
    (Class|PrimitiveComponent|CopyArrayOfMoveIgnoreComponents (Variables|Default|Gettexttrigger))
    (Rendering|Material|SetMaterial (Variables|Default|GetLight) 0 "/Game/Blueprints/KeypadSystem/Meterials/GreenGlow.GreenGlow")
    (else
      (bind _returnvalue (UserInterface|CreateWidget "/Game/Blueprints/Messages/KeycardDoor.KeycardDoor_C"))
      (UserInterface|Viewport|AddtoViewport _returnvalue 0))))

(event OnComponentEndOverlap(texttrigger)
  (params (OverlappedComponent :type Primitive%20Component%20Object%20Reference) (OtherActor :type Actor%20Object%20Reference) (OtherComp :type Primitive%20Component%20Object%20Reference) (OtherBodyIndex :type Integer))
  (bind _foundwidgets (Widget|GetAllWidgetsOfClass "/Game/Blueprints/Messages/KeycardDoor.KeycardDoor_C" true))
  (Widget|RemovefromParent _foundwidgets))

(fn ConstructionScript)