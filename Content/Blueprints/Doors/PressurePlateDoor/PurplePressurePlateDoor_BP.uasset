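; Purple pressure-plate door that opens once enough purple switches are active.
; SwtichActivated and SwitchDiactivated adjust a switch counter, playing the DoorActivation timeline to move DoorSmallA on Z at the threshold, otherwise reversing it.
; Entering Texttrigger while under the threshold shows a PressureplateDoor widget, and leaving removes widgets of that class.
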(event OnComponentBeginOverlap(Trigger)
  (params (OverlappedComponent :type Primitive%20Component%20Object%20Reference) (OtherActor :type Actor%20Object%20Reference) (OtherComp :type Primitive%20Component%20Object%20Reference) (OtherBodyIndex :type Integer) (bFromSweep :type Boolean) (SweepResult :type Hit%20Result%20Structure%20%28by%20ref%29)))

(event OnComponentBeginOverlap(texttrigger)
  (params (OverlappedComponent :type Primitive%20Component%20Object%20Reference) (OtherActor :type Actor%20Object%20Reference) (OtherComp :type Primitive%20Component%20Object%20Reference) (OtherBodyIndex :type Integer) (bFromSweep :type Boolean) (SweepResult :type Hit%20Result%20Structure%20%28by%20ref%29))
  (if (>= (Variables|Default|GetPurplePressureSwitch) (Variables|Default|GetPurpleSwitch))
    (Class|PrimitiveComponent|CopyArrayOfMoveIgnoreComponents (Variables|Default|Gettexttrigger))
    (else
      (bind _returnvalue (UserInterface|CreateWidget "/Game/Blueprints/Messages/PressureplateDoor.PressureplateDoor_C"))
      (UserInterface|Viewport|AddtoViewport _returnvalue 0))))

(event OnComponentEndOverlap(texttrigger)
  (params (OverlappedComponent :type Primitive%20Component%20Object%20Reference) (OtherActor :type Actor%20Object%20Reference) (OtherComp :type Primitive%20Component%20Object%20Reference) (OtherBodyIndex :type Integer))
  (bind _foundwidgets (Widget|GetAllWidgetsOfClass "/Game/Blueprints/Messages/PressureplateDoor.PressureplateDoor_C" true))
  (Widget|RemovefromParent _foundwidgets))

(event Custom|SwtichActivated
  (Math|Integer|IncrementInt (Variables|Default|GetPurplePressureSwitch)
    (:%20%20
      (if (>= (Variables|Default|GetPurplePressureSwitch) (Variables|Default|GetPurpleSwitch))
        (bind _doorpos (Timeline|DoorActivation Play)
          (:Update
            (Transformation|SetRelativeLocation (Variables|Default|GetDoor_Small_A) (Math|Vector|MakeVector 0.0 0.0 _doorpos) false false)))
        (else
          (Timeline|DoorActivation Reverse))))))

(event Custom|SwitchDiactivated
  (Math|Integer|DecrementInt (Variables|Default|GetPurplePressureSwitch)
    (:%20%20
      (if (>= (Variables|Default|GetPurplePressureSwitch) (Variables|Default|GetPurpleSwitch))
        (bind _doorpos (Timeline|DoorActivation Play)
          (:Update
            (Transformation|SetRelativeLocation (Variables|Default|GetDoor_Small_A) (Math|Vector|MakeVector 0.0 0.0 _doorpos) false false)))
        (else
          (Timeline|DoorActivation Reverse))))))

(fn ConstructionScript)