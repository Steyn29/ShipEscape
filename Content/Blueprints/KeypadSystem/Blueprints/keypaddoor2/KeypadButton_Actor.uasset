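; Clickable keypad button actor that forwards presses to its owning keypad actor.
; Clicking passes the button's text with confirm and backspace flags to the keypad's ButtonEntered.
; Hovering swaps the button mesh to gold, while cursor exit or ResetButtons restores steel.
; The construction script shows the configured text on the button's label.
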(event OnBeginCursorOver(button)
  (params (TouchedComponent :type Primitive%20Component%20Object%20Reference))
  ;[1 1 1] Hovered and unhovered
  (Rendering|Material|SetMaterial (Variables|Default|Getbutton) 0 "/Game/StarterContent/Materials/M_Metal_Gold.M_Metal_Gold"))

(event OnEndCursorOver(button)
  (params (TouchedComponent :type Primitive%20Component%20Object%20Reference))
  ;[1 1 1] Hovered and unhovered
  (Rendering|Material|SetMaterial (Variables|Default|Getbutton) 0 "/Game/StarterContent/Materials/M_Metal_Steel.M_Metal_Steel"))

(event OnClicked(button)
  (params (TouchedComponent :type Primitive%20Component%20Object%20Reference) (ButtonPressed :type Key%20Structure :default "None"))
  ;[1 1 1] On Button Clicked event
  (Default|ButtonEntered (Variables|Default|GetKeypadActorRef) (Variables|Default|GetnoText) (Variables|Default|GetConfirmedButton?) (Variables|Default|GetBackspaceButton?)))

(event Custom|Reset%20Buttons
  ;[1 1 1] Hovered and unhovered
  (Rendering|Material|SetMaterial (Variables|Default|Getbutton) 0 "/Game/StarterContent/Materials/M_Metal_Steel.M_Metal_Steel"))

(fn ConstructionScript
  ;[1 1 1] Setting Text on Button
  (Rendering|Components|TextRender|SetText (Variables|Default|GetButtonNumber) (Variables|Default|GetnoText)))