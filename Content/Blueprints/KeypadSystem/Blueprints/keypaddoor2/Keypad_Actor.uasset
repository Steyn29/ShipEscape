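; Keypad actor where the player enters a passcode on clickable 3D buttons to trigger a success event on a target.
; Overlap volumes show an interact prompt and register the keypad with the third-person character; interacting blends the view to the keypad camera and enables mouse events.
; Child button actors feed digits, backspace and confirm into a text render, checked against the code.
; Results show text, light and sound feedback, then either reset or release the player.
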(event OnComponentBeginOverlap(CollisionBox)
  (params (OverlappedComponent :type Primitive%20Component%20Object%20Reference) (OtherActor :type Actor%20Object%20Reference) (OtherComp :type Primitive%20Component%20Object%20Reference) (OtherBodyIndex :type Integer) (bFromSweep :type Boolean) (SweepResult :type Hit%20Result%20Structure%20%28by%20ref%29))
  ;[1 1 1] On overlap Events Set player reference
  (if (== OtherActor (Game|Player|GetPlayerPawn 0))
    (bind _asbp_third_person_character (Utilities|Casting|CastToBP_ThirdPersonCharacter OtherActor))
    (Variables|/Game/ThirdPerson/Blueprints/BP_ThirdPersonCharacter.BP_ThirdPersonCharacter_C|SetKeypadInteractActor _asbp_third_person_character self)
    (Variables|Default|SetPlayer%20ref _asbp_third_person_character)))

(event OnComponentEndOverlap(CollisionBox)
  (params (OverlappedComponent :type Primitive%20Component%20Object%20Reference) (OtherActor :type Actor%20Object%20Reference) (OtherComp :type Primitive%20Component%20Object%20Reference) (OtherBodyIndex :type Integer))
  ;[1 1 1] On overlap Events Set player reference
  (if (== OtherActor (Game|Player|GetPlayerPawn 0))
    (bind _asbp_third_person_character (Utilities|Casting|CastToBP_ThirdPersonCharacter OtherActor))
    (Variables|/Game/ThirdPerson/Blueprints/BP_ThirdPersonCharacter.BP_ThirdPersonCharacter_C|SetKeypadInteractActor _asbp_third_person_character 0)
    (Variables|Default|SetPlayer%20ref 0)))

(event OnComponentBeginOverlap(TextCollider)
  (params (OverlappedComponent :type Primitive%20Component%20Object%20Reference) (OtherActor :type Actor%20Object%20Reference) (OtherComp :type Primitive%20Component%20Object%20Reference) (OtherBodyIndex :type Integer) (bFromSweep :type Boolean) (SweepResult :type Hit%20Result%20Structure%20%28by%20ref%29))
  (bind _returnvalue (UserInterface|CreateWidget "/Game/Blueprints/Messages/PressEtoInteract_Widget.PressEtoInteract_Widget_C"))
  (UserInterface|Viewport|AddtoViewport _returnvalue 0))

(event OnComponentEndOverlap(TextCollider)
  (params (OverlappedComponent :type Primitive%20Component%20Object%20Reference) (OtherActor :type Actor%20Object%20Reference) (OtherComp :type Primitive%20Component%20Object%20Reference) (OtherBodyIndex :type Integer))
  (bind _foundwidgets (Widget|GetAllWidgetsOfClass "/Game/Blueprints/Messages/PressEtoInteract_Widget.PressEtoInteract_Widget_C" true))
  (Widget|RemovefromParent _foundwidgets))

(event Custom|On%20Interacted
  (bind _returnvalue (Game|GetPlayerController 0))
  (bind _enteredcodetext (Variables|Default|GetEnteredCodeText))
  ;[1 1 1] On player interacted with keypad. Camera view is smoothly switched to show the keypad. Mouse events turned on for 3d objects in the game
  (Game|Player|SetViewTargetwithBlend (Game|GetPlayerController 0) (Components|GetOwner (Variables|Default|GetCamera)) 0.4 "VTBlend_Linear" 0.0 false)
  (bind _output_get (Variables|/Script/Engine.PlayerController|SetbShowMouseCursor _returnvalue true))
  (bind _output_get_2 (Variables|/Script/Engine.PlayerController|SetbEnableClickEvents _returnvalue _output_get))
  (Variables|/Script/Engine.PlayerController|SetbEnableMouseOverEvents _returnvalue _output_get_2)
  (Rendering|Components|TextRender|SetText _enteredcodetext (Utilities|Text|MakeLiteralText (Utilities|Text|ToText(String) (Utilities|String|GetSubstring (Utilities|String|MakeLiteralString "..........") 0 (Utilities|String|Len (Variables|Default|GetKeypad%20Code))))))
  (Rendering|Components|TextRender|SetTextRenderColor _enteredcodetext (Math|Color|MakeColor 1 1 1 255))
  (bind _output_get_3 (Variables|Default|SetButtonsArray (Utilities|Array|MakeArray (Variables|Default|GetButton1) (Variables|Default|GetButton2) (Variables|Default|GetButton3) (Variables|Default|GetButton4) (Variables|Default|GetButton5) (Variables|Default|GetButton6) (Variables|Default|GetButton7) (Variables|Default|GetButton8) (Variables|Default|GetButton9) (Variables|Default|GetButtonBack) (Variables|Default|GetButton0) (Variables|Default|GetButtonEnter))))
  (for _array_element _output_get_3
    (bind _askeypad_button_actor (Utilities|Casting|CastToKeypadButton_Actor (Variables|/Script/Engine.ChildActorComponent|GetChildActor _array_element)))
    (Variables|/Game/Blueprints/KeypadSystem/Blueprints/keypaddoor2/KeypadButton_Actor.KeypadButton_Actor_C|SetKeypadActorRef _askeypad_button_actor self)))

(event Custom|Initiate
  (bind _returnvalue (Game|GetPlayerController 0))
  (bind _enteredcodetext (Variables|Default|GetEnteredCodeText))
  ;[1 1 1] On player interacted with keypad. Camera view is smoothly switched to show the keypad. Mouse events turned on for 3d objects in the game
  (bind _output_get (Variables|/Script/Engine.PlayerController|SetbShowMouseCursor _returnvalue true))
  (bind _output_get_2 (Variables|/Script/Engine.PlayerController|SetbEnableClickEvents _returnvalue _output_get))
  (Variables|/Script/Engine.PlayerController|SetbEnableMouseOverEvents _returnvalue _output_get_2)
  (Rendering|Components|TextRender|SetText _enteredcodetext (Utilities|Text|MakeLiteralText (Utilities|Text|ToText(String) (Utilities|String|GetSubstring (Utilities|String|MakeLiteralString "..........") 0 (Utilities|String|Len (Variables|Default|GetKeypad%20Code))))))
  (Rendering|Components|TextRender|SetTextRenderColor _enteredcodetext (Math|Color|MakeColor 1 1 1 255))
  (bind _output_get_3 (Variables|Default|SetButtonsArray (Utilities|Array|MakeArray (Variables|Default|GetButton1) (Variables|Default|GetButton2) (Variables|Default|GetButton3) (Variables|Default|GetButton4) (Variables|Default|GetButton5) (Variables|Default|GetButton6) (Variables|Default|GetButton7) (Variables|Default|GetButton8) (Variables|Default|GetButton9) (Variables|Default|GetButtonBack) (Variables|Default|GetButton0) (Variables|Default|GetButtonEnter))))
  (for _array_element _output_get_3
    (bind _askeypad_button_actor (Utilities|Casting|CastToKeypadButton_Actor (Variables|/Script/Engine.ChildActorComponent|GetChildActor _array_element)))
    (Variables|/Game/Blueprints/KeypadSystem/Blueprints/keypaddoor2/KeypadButton_Actor.KeypadButton_Actor_C|SetKeypadActorRef _askeypad_button_actor self)))

(event Custom|Button%20entered
  (params (Value :type Text) (Confirmed? :type Boolean) (Backspace :type Boolean))
  (bind _enteredcodetext (Variables|Default|GetEnteredCodeText))
  ;[1 1 1] Event called when button is pressed
  (if Confirmed?
    (CallFunction|OnConfirm)
    (elif Backspace
      (CallFunction|BackSpace)
      (elif (Variables|Default|GetCan%20enter)
        (Audio|PlaySound2D "/Engine/VREditor/Sounds/UI/Object_Snaps_To_Grid.Object_Snaps_To_Grid" 1.0 1.0 0.0 0 0)
        (Rendering|Components|TextRender|SetText _enteredcodetext (Utilities|Text|ToText(String) (Utilities|String|Replace (Utilities|String|ToString(Text) (Variables|/Script/Engine.TextRenderComponent|GetText (Variables|Default|GetEnteredCodeText))) (Utilities|String|GetSubstring (Utilities|String|MakeLiteralString "..........") 0 (Utilities|String|Len (Variables|Default|GetKeypad%20Code))))))
        (Rendering|Components|TextRender|SetText _enteredcodetext (Utilities|Text|ToText(String) (Utilities|String|Append (Utilities|String|ToString(Text) (Variables|/Script/Engine.TextRenderComponent|GetText (Variables|Default|GetEnteredCodeText))) (Utilities|String|ToString(Text) Value))))
        (Rendering|Components|TextRender|SetTextRenderColor (Variables|Default|GetEnteredCodeText) (Math|Color|MakeColor 255 255 255 255))))))

(event Custom|BackSpace
  (bind _enteredcodetext (Variables|Default|GetEnteredCodeText))
  (bind _text (Variables|/Script/Engine.TextRenderComponent|GetText _enteredcodetext))
  (bind _returnvalue (Utilities|String|ToString(Text) _text))
  ;[1 1 1] on backspace use substring to remove last character
  (Rendering|Components|TextRender|SetText _enteredcodetext (Utilities|Text|ToText(String) (Utilities|String|GetSubstring _returnvalue 0 (- (Utilities|String|Len _returnvalue) 1)))))

(event Custom|OnConfirm
  (bind _returnvalue (Game|GetPlayerController 0))
  (bind _returnvalue_2 (Game|GetPlayerController 0))
  (bind _enteredcodetext (Variables|Default|GetEnteredCodeText))
  (bind _enteredcodetext_2 (Variables|Default|GetEnteredCodeText))
  ;[1 1 1] On Confirm button pressed
  (if (Utilities|Enum|Equal(Enum) (Variables|Default|GetKeypad%20Code) (Utilities|String|ToString(Text) (Variables|/Script/Engine.TextRenderComponent|GetText (Variables|Default|GetEnteredCodeText))))
    ;;[0.06363 1 0.0398] If passcode is correct, then show feedback after delay,  back to third person view and destroy collider
    (Utilities|FlowControl|Sequence
      (:then_0
        (Rendering|Components|TextRender|SetText _enteredcodetext_2 (Utilities|Text|MakeLiteralText "Correct Passcode"))
        (Rendering|Components|TextRender|SetTextRenderColor _enteredcodetext_2 (Math|Color|MakeColor 0 255 0 255))
        (Rendering|Material|SetMaterial (Variables|Default|GetLight) 0 "/Game/Blueprints/KeypadSystem/Meterials/GreenGlow.GreenGlow")
        (Utilities|FlowControl|RetriggerableDelay 2.0)
        (bind _output_get (Variables|/Script/Engine.PlayerController|SetbShowMouseCursor _returnvalue_2 false))
        (bind _output_get_2 (Variables|/Script/Engine.PlayerController|SetbEnableMouseOverEvents _returnvalue_2 _output_get))
        (Variables|/Script/Engine.PlayerController|SetbEnableClickEvents _returnvalue_2 _output_get_2)
        (for _array_element (Variables|Default|GetButtonsArray)
          (bind _askeypad_button_actor (Utilities|Casting|CastToKeypadButton_Actor (Variables|/Script/Engine.ChildActorComponent|GetChildActor _array_element)))
          (Default|ResetButtons _askeypad_button_actor))
        (Game|Player|SetViewTargetwithBlend (Game|GetPlayerController 0) (Components|GetOwner (Variables|/Game/ThirdPerson/Blueprints/BP_ThirdPersonCharacter.BP_ThirdPersonCharacter_C|GetFollowCamera (.AsBP%20Third%20Person%20Character (Utilities|Casting|CastToBP_ThirdPersonCharacter (Game|Player|GetPlayerPawn 0))))) 0.4 "VTBlend_Linear" 0.0 false)
        (Rendering|Components|TextRender|SetText (Variables|Default|GetEnteredCodeText) (Utilities|Text|MakeLiteralText ""))
        (Input|SetInputModeGameOnly (Game|GetPlayerController 0) false)
        (Components|DestroyComponent (Variables|Default|GetCollisionBox))
        (Components|DestroyComponent (Variables|Default|GetTextCollider))
        (Class|KeypadBPI|KeypadSucessEvent(Message) (Variables|Default|GetKeypadTarget)))
      (:then_1
        (Variables|Default|SetCan%20enter false)
        (Audio|PlaySound2D "/Engine/VREditor/Sounds/UI/Camera_Shutter.Camera_Shutter" 1.0 1.0 0.0 0 0)))
    (else
      ;;[1 0 0.07252] If passcode wrong then show feedback after delay , reset keypad so use can try again
      (Utilities|FlowControl|Sequence
        (:then_0
          (Rendering|Components|TextRender|SetText _enteredcodetext (Utilities|Text|MakeLiteralText "Wrong Passcode"))
          (Rendering|Components|TextRender|SetTextRenderColor _enteredcodetext (Math|Color|MakeColor 0 0 255 255))
          (Rendering|Material|SetMaterial (Variables|Default|GetLight) 0 "/Game/Blueprints/KeypadSystem/Meterials/RedGlow.RedGlow")
          (Utilities|FlowControl|RetriggerableDelay 2.0)
          (bind _output_get_3 (Variables|/Script/Engine.PlayerController|SetbEnableMouseOverEvents _returnvalue false))
          (Variables|/Script/Engine.PlayerController|SetbEnableClickEvents _returnvalue _output_get_3)
          (for _array_element_2 (Variables|Default|GetButtonsArray)
            (bind _askeypad_button_actor_2 (Utilities|Casting|CastToKeypadButton_Actor (Variables|/Script/Engine.ChildActorComponent|GetChildActor _array_element_2)))
            (Default|ResetButtons _askeypad_button_actor_2))
          (CallFunction|Initiate)
          (Variables|Default|SetCan%20enter true))
        (:then_1
          (Variables|Default|SetCan%20enter false)
          (Audio|PlaySound2D "/Engine/VREditor/Sounds/UI/Invalid_Action.Invalid_Action" 1.0 1.0 0.0 0 0))))))

(fn ConstructionScript)