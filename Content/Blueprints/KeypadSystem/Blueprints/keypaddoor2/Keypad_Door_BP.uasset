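; Keypad-locked door actor that prompts on approach and opens by being removed.
; Overlapping its Box creates an UnlockKeypadToEnter widget, and ending the overlap removes top-level widgets of that class, with no check on the overlapping actor.
; KeypadSucessEvent destroys the Door and Box components, clearing the way and ending the prompt trigger; the event is not called within this Blueprint.
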(event OnComponentBeginOverlap(Box)
  (params (OverlappedComponent :type Primitive%20Component%20Object%20Reference) (OtherActor :type Actor%20Object%20Reference) (OtherComp :type Primitive%20Component%20Object%20Reference) (OtherBodyIndex :type Integer) (bFromSweep :type Boolean) (SweepResult :type Hit%20Result%20Structure%20%28by%20ref%29))
  ;[1 1 1] Show text to the object
  (bind _returnvalue (UserInterface|CreateWidget "/Game/Blueprints/Messages/UnlockKeypadToEnter.UnlockKeypadToEnter_C"))
  (UserInterface|Viewport|AddtoViewport _returnvalue 0))

(event OnComponentEndOverlap(Box)
  (params (OverlappedComponent :type Primitive%20Component%20Object%20Reference) (OtherActor :type Actor%20Object%20Reference) (OtherComp :type Primitive%20Component%20Object%20Reference) (OtherBodyIndex :type Integer))
  ;[1 1 1] Show text to the object
  (bind _foundwidgets (Widget|GetAllWidgetsOfClass "/Game/Blueprints/Messages/UnlockKeypadToEnter.UnlockKeypadToEnter_C" true))
  (Widget|RemovefromParent _foundwidgets))

(event EventKeypadSucessEvent
  (Components|DestroyComponent (Variables|Default|GetDoor)))

(fn ConstructionScript)